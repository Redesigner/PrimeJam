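; BP_PrimePlayerController is the player controller that creates the player's HUD and a targeting reticle widget.
; On BeginPlay it adds both widgets to the viewport, hides the mouse cursor and sizes the reticle.
; On possess it binds to the pawn's TargetingComponent cursor-position event and moves the reticle to each new position with DPI scaling removed.
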(event Custom|OnCursorPositionChanged_Event
  (params (Position :type Vector%202D%20Structure))
  (Class|UserWidget|SetPositioninViewport (Variables|Default|GetReticle%20Widget) Position true))

(event EventBeginPlay
  (Utilities|FlowControl|Sequence
    (:then_0
      (bind _returnvalue (UserInterface|CreateWidget "/Game/UI/Reticle/WBP_TargetingReticle.WBP_TargetingReticle_C"))
      (bind _output_get (Variables|Default|SetReticle%20Widget _returnvalue))
      (UserInterface|Viewport|AddtoViewport _output_get 0)
      (Variables|Default|SetbShowMouseCursor false)
      (Class|UserWidget|SetDesiredSizeinViewport _output_get "(X=128.000000,Y=128.000000)"))
    (:then_1
      (bind _returnvalue_2 (UserInterface|CreateWidget "/Game/UI/HUD/WBP_HUDBase.WBP_HUDBase_C"))
      (UserInterface|Viewport|AddtoViewport _returnvalue_2 0))))

(event EventPossess
  (params (PossessedPawn :type Pawn%20Object%20Reference))
  (EventDispatchers|AssignOnCursorPositionChanged (Actor|GetComponentbyClass PossessedPawn "/Script/PrimeJam.TargetingComponent") (delegate Custom|OnCursorPositionChanged_Event)))

(fn ConstructionScript)